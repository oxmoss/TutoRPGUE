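; Shop owner NPC that flags when the field player is in talking range and shows a prompt.
; Overlapping its interaction box sets TalkShop on the RPG game instance and mirrors it to Talk.
; Tick passes these to helpers for a camera-facing text prompt and collision box blinking.
; Local graphs BlinkOverlapOnDebug and SetupTextTooltip hold similar logic, including debug-only box display, but Tick calls differently named helpers.
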(event OnComponentBeginOverlap(interactionBox)
  (params (OverlappedComponent :type Primitive%20Component%20Object%20Reference) (OtherActor :type Actor%20Object%20Reference) (OtherComp :type Primitive%20Component%20Object%20Reference) (OtherBodyIndex :type Integer) (bFromSweep :type Boolean) (SweepResult :type Hit%20Result%20Structure%20%28by%20ref%29))
  (Utilities|Casting|CastToFieldPlayer OtherActor)
  (bind _asrpggame_instance (Utilities|Casting|CastToRPGGameInstance (Game|GetGameInstance)))
  (bind _output_get (Variables|/Script/RPG.RPGGameInstance|SetTalkShop _asrpggame_instance true))
  (Variables|Default|Settalk _output_get))

(event OnComponentEndOverlap(interactionBox)
  (params (OverlappedComponent :type Primitive%20Component%20Object%20Reference) (OtherActor :type Actor%20Object%20Reference) (OtherComp :type Primitive%20Component%20Object%20Reference) (OtherBodyIndex :type Integer))
  (Utilities|Casting|CastToFieldPlayer OtherActor)
  (bind _asrpggame_instance (Utilities|Casting|CastToRPGGameInstance (Game|GetGameInstance)))
  (bind _output_get (Variables|/Script/RPG.RPGGameInstance|SetTalkShop _asrpggame_instance false))
  (Variables|Default|Settalk _output_get))

(event EventTick
  (params (DeltaSeconds :type Float%20%28single-precision%29))
  (bind _asrpggame_instance (Utilities|Casting|CastToRPGGameInstance (Game|GetGameInstance)))
  (CallFunction|TextFollowCamera (Variables|/Script/RPG.RPGGameInstance|GetTalkShop _asrpggame_instance) (Variables|Default|GetTextRender))
  (CallFunction|BlinkBoxCollision DeltaSeconds (Variables|Default|Getblink) (Variables|Components|GetinteractionBox)))

(fn ConstructionScript)