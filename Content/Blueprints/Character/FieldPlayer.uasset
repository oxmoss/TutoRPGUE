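; FieldPlayer is the field player Blueprint, and its graph holds debug hotkeys and the pause menu input.
; V toggles the debug flag on BP_RPGGameMode through a FlipFlop, and C calls that game mode's TestCombat.
; Releasing P pauses the game, opens a Pause_Main widget targeting the first party member from RPGGameInstance, and shows the mouse cursor.
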(event Input|KeyboardEvents|V
  (params (Key :type Key%20Structure :default "AnyKey"))
  ;[1 1 1] [DEBUG] V key Enable debug on
  (:Pressed
    (bind _asbp_rpggame_mode (Utilities|Casting|CastToBP_RPGGameMode (Game|GetGameMode)))
    (bind _isa (Utilities|FlowControl|FlipFlop)
      (:A
        _)
      (:B
        _))
    (bind _output_get (Variables|/Script/RPG.RPGGameMode|SetdebugEnabled _asbp_rpggame_mode _isa))
    (if _output_get
      (Development|PrintString "Debug enabled" true true "(R=0.000000,G=0.219608,B=1.000000,A=1.000000)" 3.0)
      (else
        (Development|PrintString "Debug disabled" true true "(R=1.000000,G=0.000000,B=0.000000,A=1.000000)" 3.0)))))

(event Input|KeyboardEvents|P
  (params (Key :type Key%20Structure :default "AnyKey"))
  ;[1 1 1] Pause menu TODO
  (:Released
    (Game|SetGamePaused true)
    (bind _returnvalue (UserInterface|CreateWidget "/Game/Blueprints/UI/Pause/Pause_Main.Pause_Main_C"))
    (bind _asrpggame_instance (Utilities|Casting|CastToRPGGameInstance (Game|GetGameInstance)))
    (Variables|/Game/Blueprints/UI/Pause/Pause_Main.Pause_Main_C|SetCharacterTarget _returnvalue (Utilities|Array|Get(acopy) (Variables|/Script/RPG.RPGGameInstance|GetPartyMembers _asrpggame_instance)))
    (UserInterface|Viewport|AddtoViewport _returnvalue 0)
    (Variables|/Script/Engine.PlayerController|SetbShowMouseCursor (Game|GetPlayerController 0) true)))

(event Input|KeyboardEvents|C
  (params (Key :type Key%20Structure :default "AnyKey"))
  ;[1 1 1] [DEBUG] C key launch TestCombat
  (:Pressed
    (bind _asbp_rpggame_mode (Utilities|Casting|CastToBP_RPGGameMode (Game|GetGameMode)))
    (Class|RPGGameMode|TestCombat _asbp_rpggame_mode)))

(fn ConstructionScript)