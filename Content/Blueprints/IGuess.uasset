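; IGuess holds helper functions for debug collision display and camera-facing text in an RPG.
; BlinkBoxCollision shows a collision box while the game mode's debug flag is on, toggling it every BlinkLength seconds during player pawn overlap via a by-reference delta-time accumulator.
; TextFollowCamera sets a text component's visibility and, when visible, rotates it toward the player camera.
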(fn BlinkBoxCollision
  (params (DeltaSeconds :type Float%20%28single-precision%29) (Blink :type Float%20%28single-precision%29%20%28by%20ref%29) (CollisionBox :type Box%20Component%20Object%20Reference))
  (bind _returnvalue (+ DeltaSeconds Blink))
  (bind _asbp_rpggame_mode (Utilities|Casting|CastToBP_RPGGameMode (Game|GetGameMode)))
  (if (Variables|/Script/RPG.RPGGameMode|GetdebugEnabled _asbp_rpggame_mode)
    (if (Collision|IsOverlappingActor CollisionBox (Game|Player|GetPlayerPawn 0) :!class /Script/Engine.PrimitiveComponent)
      (|SetBy-RefVar Blink _returnvalue)
      (if (>= _returnvalue (LocalVariables|GetBlinkLength))
        (|SetBy-RefVar Blink 0.0)
        (if (Variables|/Script/Engine.SceneComponent|GetbHiddenInGame CollisionBox)
          (Development|SetHiddeninGame CollisionBox false false)
          (else
            (Development|SetHiddeninGame CollisionBox true false))))
      (else
        (Development|SetHiddeninGame CollisionBox false false)))
    (else
      (Development|SetHiddeninGame CollisionBox true false))))

(fn TextFollowCamera
  (params (Visibility :type Boolean) (Text :type Text%20Render%20Component%20Object%20Reference))
  (if Visibility
    (Rendering|SetVisibility Text true true)
    (Transformation|SetWorldRotation Text (Math|Rotator|FindLookatRotation (Transformation|GetWorldLocation Text) (Transformation|GetActorLocation (Game|GetPlayerCameraManager 0))) false false)
    (else
      (Rendering|SetVisibility Text false true))))